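; RTS camera actor that becomes the first player's view target on BeginPlay and pans when the mouse nears a screen edge.
; Tick calls four directional functions that offset the root component along X for left/right and Y for up/down.
; Speed ramps linearly across the outer five percent of the viewport using clamped normalized mouse position.
; Movement is per frame, without delta-time scaling or bounds.
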(event `self.ReceiveBeginPlay`
  (`PlayerController.SetViewTargetWithBlend` (`GameplayStatics.GetPlayerController` 0) self 0.0 "VTBlend_Linear" 0.0 false))

(event `self.ReceiveTick`
  (params (DeltaSeconds :type "Float (single-precision)"))
  (`self.MoveLeft`)
  (`self.MoveRight`)
  (`self.MoveDown`)
  (`self.MoveUp`))

(fn `MoveDown`
  (bind (_returnvalue_x _returnvalue_y) (`KismetMathLibrary.BreakVector2D` (`WidgetLayoutLibrary.GetViewportSize`)))
  (bind _returnvalue (`WidgetLayoutLibrary.GetMousePositionOnViewport`))
  (`SceneComponent.K2_AddRelativeLocation` (`self.DefaultSceneRoot`) (* (0.0 -50.0 0.0) (`KismetMathLibrary.FClamp` (`KismetMathLibrary.NormalizeToRange` (`.Y` (`KismetMathLibrary.BreakVector2D` _returnvalue)) (* _returnvalue_y 0.95) _returnvalue_y))) false false))

(fn `MoveLeft`
  (bind _returnvalue_x (`KismetMathLibrary.BreakVector2D` (`WidgetLayoutLibrary.GetViewportSize`)))
  (bind _returnvalue (`WidgetLayoutLibrary.GetMousePositionOnViewport`))
  (`SceneComponent.K2_AddRelativeLocation` (`self.DefaultSceneRoot`) (* (50.0 0.0 0.0) (- 1.0 (`KismetMathLibrary.FClamp` (`KismetMathLibrary.NormalizeToRange` (`KismetMathLibrary.BreakVector2D` _returnvalue) 0.0 (* _returnvalue_x 0.05)) 0.0 1.0))) false false))

(fn `MoveRight`
  (bind _returnvalue_x (`KismetMathLibrary.BreakVector2D` (`WidgetLayoutLibrary.GetViewportSize`)))
  (bind _returnvalue (`WidgetLayoutLibrary.GetMousePositionOnViewport`))
  (`SceneComponent.K2_AddRelativeLocation` (`self.DefaultSceneRoot`) (* (-50.0 0.0 0.0) (`KismetMathLibrary.FClamp` (`KismetMathLibrary.NormalizeToRange` (`KismetMathLibrary.BreakVector2D` _returnvalue) (* _returnvalue_x 0.95) _returnvalue_x) 0.0)) false false))

(fn `MoveUp`
  (bind (_returnvalue_x _returnvalue_y) (`KismetMathLibrary.BreakVector2D` (`WidgetLayoutLibrary.GetViewportSize`)))
  (bind _returnvalue (`WidgetLayoutLibrary.GetMousePositionOnViewport`))
  (`SceneComponent.K2_AddRelativeLocation` (`self.DefaultSceneRoot`) (* (0.0 50.0 0.0) (- 1.0 (`KismetMathLibrary.FClamp` (`KismetMathLibrary.NormalizeToRange` (`.Y` (`KismetMathLibrary.BreakVector2D` _returnvalue)) 0.0 (* 0.05 _returnvalue_y))))) false false))

(fn `UserConstructionScript`)